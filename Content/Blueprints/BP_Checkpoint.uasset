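; BP_Checkpoint is a checkpoint actor that sets the player's respawn point and marks itself with a flag.
; When an overlapping actor's instigator is BP_Player, it stores the RespawnLocation transform in BP_GameInstance and sets CheckpointOn.
; It then loops over all checkpoints, hiding each flag while re-showing its own and playing the checkpoint sound on every iteration, so only its flag remains visible.
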(event OnComponentBeginOverlap(s)
  (params (OverlappedComponent :type Primitive%20Component%20Object%20Reference) (OtherActor :type Actor%20Object%20Reference) (OtherComp :type Primitive%20Component%20Object%20Reference) (OtherBodyIndex :type Integer) (bFromSweep :type Boolean) (SweepResult :type Hit%20Result%20Structure%20%28by%20ref%29))
  (Utilities|Casting|CastToBP_Player (Game|GetInstigator OtherActor))
  (bind _asbp_game_instance (Utilities|Casting|CastToBP_GameInstance (Game|GetGameInstance)))
  (Variables|/Game/Blueprints/BP_GameInstance.BP_GameInstance_C|SetRespawnTransform _asbp_game_instance (Transformation|GetWorldTransform (Variables|Default|GetRespawnLocation)))
  (Variables|/Game/Blueprints/BP_GameInstance.BP_GameInstance_C|SetCheckpointOn _asbp_game_instance true)
  (bind _outactors (Actor|GetAllActorsOfClass "BP_Checkpoint_C"))
  (for _array_element _outactors
    (Development|SetHiddeninGame (Variables|BP_Checkpoint_C|GetFlag _array_element) true false)
    (Audio|PlaySoundatLocation "/Game/Audio/checkpoint.checkpoint" "0, 0, 0" "0, 0, 0" 0.1 1.0 0.0 0 0 0 0)
    (Development|SetHiddeninGame (Variables|Default|GetFlag) false false)))

(fn ConstructionScript)