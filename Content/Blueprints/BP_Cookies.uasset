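; BP_Cookies is a collectible cookie pickup that spins its static mesh every tick by RotationSpeed, without delta-time scaling.
; Any overlap with PickUpRadius increments the Cookies count on BP_GameInstance and prints it, without checking which actor overlapped.
; It then writes the new count to the CookiesAmount text in BP_Player's HUD and destroys itself.
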(event OnComponentBeginOverlap(PickUpRadius)
  (params (OverlappedComponent :type Primitive%20Component%20Object%20Reference) (OtherActor :type Actor%20Object%20Reference) (OtherComp :type Primitive%20Component%20Object%20Reference) (OtherBodyIndex :type Integer) (bFromSweep :type Boolean) (SweepResult :type Hit%20Result%20Structure%20%28by%20ref%29))
  (bind _asbp_game_instance (Utilities|Casting|CastToBP_GameInstance (Game|GetGameInstance)))
  (bind _result (Math|Integer|IncrementInt (Variables|/Game/Blueprints/BP_GameInstance.BP_GameInstance_C|GetCookies _asbp_game_instance))
    (:%20%20
      (Development|PrintString (Utilities|String|ToString(Integer) _result))
      (bind _asbp_player (Utilities|Casting|CastToBP_Player (Game|GetPlayerCharacter 0)))
      (Rendering|Components|TextRender|SetText (Variables|/Game/UI/WB_PlayerHud.WB_PlayerHud_C|GetCookiesAmount (Variables|/Game/Blueprints/BP_Player.BP_Player_C|GetHudReference _asbp_player)) (Utilities|Text|ToText(String) (Utilities|String|ToString(Integer) _result)))
      (Actor|DestroyActor))))

(event EventTick
  (params (DeltaSeconds :type Float%20%28single-precision%29))
  (Transformation|AddRelativeRotation (Variables|Default|GetStaticMesh) (Math|Rotator|MakeRotator 0.0 0.0 (Variables|Default|GetRotationSpeed)) false false))

(fn ConstructionScript)